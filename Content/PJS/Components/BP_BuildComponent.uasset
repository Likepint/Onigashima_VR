(event `self.ReceiveBeginPlay`
  (bind _asbp_ccharacter_pjs (cast `/Game/PJS/Characters/BP_CCharacter_PJS` (`self.GetOwner`)))
  (set `self.UserRef` _asbp_ccharacter_pjs))

(event `BuildDelay`
  (bind _outline (`self.OutLine`))
  (if (`self.bOnBuildMode`)
    (`KismetSystemLibrary.Delay` 0.01)
    (`self.BuildCycle`)
    (else
      (set `self.bOnBuildMode` false :!label _label)
      (set `self.bCanBuild` false)
      (`/Engine/EditorBlueprintResources/StandardMacros.IsValid` _outline
        (:`Is Valid`
          (`/Game/PJS/Characters/BP_CCharacter_PJS.DestroyComponent` (`self.UserRef`) _outline))))))

(event `StopBuildMode`
  (goto _label))

(event `LaunchBuildMode`
  (if (`self.bOnBuildMode`)
    (`self.StopBuildMode`)
    (else
      (set `self.bOnBuildMode` true)
      (`self.BuildCycle`))))

(fn `BuildCycle`
  (bind _camera (`self.Camera`))
  (bind (_buildtransform_location _buildtransform_rotation _buildtransform_scale) (`KismetMathLibrary.BreakTransform` (`self.BuildTransform`)))
  (bind _outline (`self.OutLine`))
  (bind _returnvalue (`SceneComponent.K2_GetComponentLocation` _camera))
  (bind _returnvalue_2 (`SceneComponent.GetForwardVector` _camera))
  (bind (_outhit _returnvalue_3) (`KismetSystemLibrary.LineTraceSingle` (+ _returnvalue (* _returnvalue_2 350.0)) (+ _returnvalue (* _returnvalue_2 1000.0)) "TraceTypeQuery1"))
  (if _returnvalue_3
    (bind (_bblockinghit _binitialoverlap _time _distance _location _impactpoint _normal _impactnormal _physmat _hitactor _hitcomponent _hitbonename _bonename _hititem _elementindex _faceindex _tracestart _traceend) (`GameplayStatics.BreakHitResult` _outhit))
    (set `self.BuildTransform` (`KismetMathLibrary.MakeTransform` _impactpoint _buildtransform_rotation _buildtransform_scale))
    (`/Engine/EditorBlueprintResources/StandardMacros.IsValid` _outline
      (:`Is Valid`
        (`self.GiveBuildColor` true))
      (:`Is Not Valid`
        (`self.SpawnBuildOutLine` :!label _label)))
    (else
      (set `self.BuildTransform` (`KismetMathLibrary.MakeTransform` _traceend _buildtransform_rotation _buildtransform_scale))
      (`/Engine/EditorBlueprintResources/StandardMacros.IsValid` _outline
        (:`Is Valid`
          (`self.GiveBuildColor` false))
        (:`Is Not Valid`
          (goto _label)))))
  (`self.BuildDelay`))

(fn `GiveBuildColor`
  (params (Condition :type Boolean))
  (bind _outline (`self.OutLine`))
  (set `self.bCanBuild` false)
  (for _index (range (- (`PrimitiveComponent.GetNumMaterials` (`self.OutLine`)) 1) 1)
    (if Condition
      (`PrimitiveComponent.SetMaterial` _outline _index "/Game/PJS/Materials/MI_Green.MI_Green")
      (else
        (`PrimitiveComponent.SetMaterial` _outline _index "/Game/PJS/Materials/MI_Red.MI_Red"))))
  (`SceneComponent.K2_SetWorldTransform` (`self.OutLine`) (`self.BuildTransform`) false false))

(fn `SpawnBuildOutLine`
  (bind _returnvalue (`|AddComponentByClass` (`self.UserRef`) "/Script/Engine.StaticMeshComponent" false (`self.BuildTransform`)))
  (bind _output_get (set `self.OutLine` _returnvalue))
  (`StaticMeshComponent.SetStaticMesh` _output_get "/Game/PJS/Assets/foundation.foundation")
  (`PrimitiveComponent.SetCollisionEnabled` (`self.OutLine`) "NoCollision"))