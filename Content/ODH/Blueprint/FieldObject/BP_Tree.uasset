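; BP_Tree is a choppable tree field object that turns into a planks item after enough axe hits.
; Each actor overlap with a BP_Axe increments an overlap counter.
; Tick polls that counter and, once it reaches three, spawns BP_CItem_Planks at the static mesh's world transform and destroys the tree.
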(event `self.ReceiveActorBeginOverlap`
  (params (OtherActor :type "Actor Object Reference"))
  (cast `/Game/ODH/Blueprint/BP_Axe` OtherActor)
  (set `self.AxeOverlapCount` (+ (`self.AxeOverlapCount`) 1)))

(event `self.ReceiveTick`
  (params (DeltaSeconds :type "Float (single-precision)"))
  (if (>= (`self.AxeOverlapCount`) 3)
    (`|SpawnActorFromClass` "/Game/PJS/Crafts/BP_CItem_Planks.BP_CItem_Planks_C" (`SceneComponent.K2_GetComponentToWorld` (`self.StaticMesh`)) "Undefined" "MultiplyWithRoot" null null)
    (`self.K2_DestroyActor`)))

(fn `UserConstructionScript`)