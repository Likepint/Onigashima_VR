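; BP_Rock is a breakable rock field object that shatters after being struck by a pick.
; Each actor overlap with a BP_Pick increments a hit counter.
; Tick polls that counter and, once it reaches three, spawns BP_StoneBroken at the Scene component's transform and destroys the rock.
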(event `self.ReceiveActorBeginOverlap`
  (params (OtherActor :type "Actor Object Reference"))
  (cast `/Game/ODH/Blueprint/BP_Pick` OtherActor)
  (set `self.PickOverlapCount` (+ (`self.PickOverlapCount`) 1)))

(event `self.ReceiveTick`
  (params (DeltaSeconds :type "Float (single-precision)"))
  (if (>= (`self.PickOverlapCount`) 3)
    (`|SpawnActorFromClass` "/Game/ODH/Blueprint/FieldObject/BP_StoneBroken.BP_StoneBroken_C" (`SceneComponent.K2_GetComponentToWorld` (`self.Scene`)) "Undefined" "MultiplyWithRoot" null null)
    (`self.K2_DestroyActor`)))

(fn `UserConstructionScript`)